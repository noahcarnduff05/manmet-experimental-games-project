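; Spoon enemy for a tower defense game that follows a random "BasicPaths" spline to attack the gate.
; One timeline moves it along the spline over a set duration, while another bounces its body at a random rate.
; Damage plays hurt feedback and adds a half-health overlay, while death triggers an explosion, pays the player and notifies BP_GameManager.
; Reaching the path's end damages BP_Gate and removes the enemy.
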(event Custom|Move%20Along%20Path
  (bind _spliney (Variables|Default|GetSpliney))
  ;[1 0.6835 0.272 0.161] Initialises the timeline for the enemy - with the pathing time being the amount of seconds from Spawning to damaging the Gate. I would've preferred some kind of Units Per Second measurement for the pure logical sense that would make, but a set duration also makes it easy to tell how much time the player has to react and kill an enemy and balance based on speed and health.
  (Components|Timeline|SetPlayRate (Variables|Default|GetEnemyMoving) (/ 1.0 (Variables|Default|GetPathingTime)))
  (bind _newtrack_0 (Timeline|EnemyMoving Play)
    (:Update
      ;[0.5718 1 0.8684 0.583] Similar to the Elevator tutorial, Ziplines, and even the Bounce animation in this very Blueprint; the Actor moves along the Spline using the Timeline as a blend. A being the very beginning of the Spline (0) and B being the entirety of the Spline's length.
      (Transformation|SetActorTransform (Math|Transform|MakeTransform (Spline|GetLocationatDistanceAlongSpline _spliney (Math|Float|Lerp 0.0 (Spline|GetSplineLength _spliney) _newtrack_0) "World") (Spline|GetRotationatDistanceAlongSpline _spliney (Math|Float|Lerp 0.0 (Spline|GetSplineLength _spliney) _newtrack_0) "World") "1.000000,1.000000,1.000000")))
    (:Finished
      ;[1 0.4533 0.2517] When the Timeline is finished, the Enemy is at the end of the path and can therefore damage the Gate and destroy itself. Alternatively there could've been a state where the enemy stands and continuously hurts the Gate until being purposefully killed, but due to the nature of the Spline pathing system this would've caused a lot of overlapping and was ultimately too confusing.
      (Variables|Default|GetSpoon
        (:then
          (bind _returnvalue (Actor|GetActorOfClass "/Game/TDBlueprints/BP_Gate.BP_Gate_C"))
          (Default|HurtGate _returnvalue (Variables|Default|GetGateDamage) (Variables|Default|GetEnemyName))
          (Actor|DestroyActor)
          (bind _returnvalue_2 (Actor|GetActorOfClass "/Game/TDBlueprints/BP_GameManager.BP_GameManager_C"))
          (Default|EnemyRemoved _returnvalue_2))
        (:else)))))

(event EventBeginPlay
  ;[1 0.3072 0.2474 0.406] Initialise MaxHealth variable for enemies with over 1HP that will use a Half-Health Indicator or Healthbar.
  (Variables|Default|SetMaxHealth (Variables|Default|GetHealth))
  ;[1 0.1914 0.8895 0.219] Finds a random path for the Enemy to move along using Tags (with different types of enemies like Pizza Cutters having other paths that can be accessed with a different tag) and sets that Blueprint's Spline as a reference point.
  (bind _outactors (Actor|GetAllActorswithTag "BasicPaths"))
  (Variables|Default|SetSpliney (Actor|GetComponentbyClass (.OutItem (Utilities|Array|Random _outactors)) "/Script/Engine.SplineComponent"))
  (CallFunction|MoveAlongPath)
  ;[1 0.5625 0.01481 0.422] A timeline gives each enemy a small bounce for more lively visuals. Each enemy chooses a float within a limited range to bounce in duration to, so that crowds become more "realistic" (As realistic as living Knives and Forks can be.)
  (bind _output_get (Variables|Default|SetBounceSpeed (Math|Random|RandomFloatinRange 0.9 1.2)))
  (Components|Timeline|SetPlayRate (Variables|Default|GetTimeline) _output_get)
  (bind _bounce (Timeline|Timeline Play)
    (:Update
      (Transformation|SetRelativeLocation (Variables|Default|GetBodyBox) (Math|Vector|MakeVector 0.0 0.0 (.z (Math|Vector|Lerp(Vector) "0.000000,0.000000,180.000000" "0.000000,0.000000,260.000000" _bounce))) false false))))

(event Game|Damage|EventAnyDamage
  (params (Damage :type Float%20%28single-precision%29) (DamageType :type Damage%20Type%20Object%20Reference) (InstigatedBy :type Controller%20Object%20Reference) (DamageCauser :type Actor%20Object%20Reference))
  ;[0.1742 1 0.1335 0.13] Update Enemy's health
  (bind _output_get (Variables|Default|SetHealth (- (Variables|Default|GetHealth) Damage)))
  ;[1 0.3319 0.6767 0.214] If the health is less than or equal to 0, the process of killing the enemy will begin, otherwise a hurt sound will play for feedback and another check will be done to see if extra feedback should be given for enemies with more than 1HP.
  (if (<= _output_get 0.0)
    (Audio|Components|Audio|Stop (Variables|Default|GetTimeline))
    ;[0.647 0.3936 1 0.302] Spawn Explosion particle effect and kill sound upon defeating an enemy.
    (Effects|SpawnEmitteratLocation "/Game/StarterContent/Particles/P_Explosion.P_Explosion" (Transformation|GetWorldLocation (Variables|Default|GetHeadBox)))
    (Audio|PlaySoundatLocation "/Game/TDAudio/enemykill.enemykill" (Transformation|GetWorldLocation (Variables|Default|GetHeadBox)) "0, 0, 0" 1.0 1.0 0.0 "/Game/TDAudio/EnemyHitAtten.EnemyHitAtten" 0 0 0)
    ;[0.1382 0.8903 1 0.417] Update the player's current balance based on the designated Cash Reward, with an animation in the HUD.
    (bind _asbp_first_person_character (Utilities|Casting|CastToBP_FirstPersonCharacter (Game|GetPlayerCharacter 0)))
    (Variables|/Game/FirstPerson/Blueprints/BP_FirstPersonCharacter.BP_FirstPersonCharacter_C|Setcurrency _asbp_first_person_character (+ (Variables|/Game/FirstPerson/Blueprints/BP_FirstPersonCharacter.BP_FirstPersonCharacter_C|Getcurrency _asbp_first_person_character) (Variables|Default|GetCashReward)))
    (UserInterface|Animation|PlayAnimation (Variables|/Game/FirstPerson/Blueprints/BP_FirstPersonCharacter.BP_FirstPersonCharacter_C|GetPlayerHUD _asbp_first_person_character) (Variables|/Game/TDWidgets/UI_PlayerHUD.UI_PlayerHUD_C|GetMoneyGet (Variables|/Game/FirstPerson/Blueprints/BP_FirstPersonCharacter.BP_FirstPersonCharacter_C|GetPlayerHUD _asbp_first_person_character)) 0.0 1 "Forward" 1.0 false)
    (bind _returnvalue (Actor|GetActorOfClass "/Game/TDBlueprints/BP_GameManager.BP_GameManager_C"))
    (Default|EnemyDefeated _returnvalue)
    ;[1 0.6361 0.315 0.422] Destroys all visible components, with the Actor itself being destroyed after ample time is given for the Explosion particles.
    (Components|DestroyComponent (Variables|Default|GetBodyBox))
    (Utilities|FlowControl|Delay 3.0)
    (Actor|DestroyActor)
    (else
      (Audio|PlaySoundatLocation "/Game/TDAudio/enemyhurt.enemyhurt" (Transformation|GetWorldLocation (Variables|Default|GetHeadBox)) "0, 0, 0" 1.0 1.0 0.0 "/Game/TDAudio/EnemyHitAtten.EnemyHitAtten" 0 0 0)
      ;[1 0 0.1986 0.391] If the enemy is equal to or under half of its maximum health, an Overlay Material is applied. This can let the player strategise and prioritise different enemies in high-density waves.
      (if (<= _output_get (/ (Variables|Default|GetMaxHealth) 2.0))
        (Variables|/Script/Engine.MeshComponent|GetOverlayMaterial (Variables|Default|GetSpoon)
          (:then)
          (:else
            (Rendering|Material|SetOverlayMaterial (Variables|Default|GetSpoon) "/Game/TDMaterials/OM_HalfHealth.OM_HalfHealth" :!class /Script/Engine.MeshComponent)))))))

(fn ConstructionScript)