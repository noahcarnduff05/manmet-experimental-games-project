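; Game manager for a gate-defence wave game, running the loop of timed breaks, enemy waves and results screens.
; Breaks drive the HUD timer bar and music, then NewWave removes the shop and spawns enemies at random intervals from a weighted table.
; Defeats and other removals count toward WaveCleared, which shows results, or a cinematic final results screen when Wave equals 1.
; MakeNewWave increments the wave, spawns the shop and starts the next break.
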(event Custom|Break%20Time
  (params (Break%20Length :type Float%20%28double-precision%29))
  (Variables|BreakVars|SetInBreak true)
  (Variables|BreakVars|SetCurrentBreakLength Break%20Length)
  (bind _returnvalue (Audio|SpawnSound2D "/Game/TDAudio/Music/breakmusic.breakmusic" 0.3 1.0 0.0 0))
  (bind _output_get (Variables|Default|SetBreakMusic _returnvalue))
  (Audio|Components|Audio|FadeIn _output_get 2.0 1.0 0.0 "Linear" :!class /Script/Engine.AudioComponent)
  (bind _asbp_first_person_character (Utilities|Casting|CastToBP_FirstPersonCharacter (Game|GetPlayerCharacter 0)))
  (UserInterface|Animation|PlayAnimation (Variables|/Game/FirstPerson/Blueprints/BP_FirstPersonCharacter.BP_FirstPersonCharacter_C|GetPlayerHUD _asbp_first_person_character) (Variables|/Game/TDWidgets/UI_PlayerHUD.UI_PlayerHUD_C|GetBreakTimeStart (Variables|/Game/FirstPerson/Blueprints/BP_FirstPersonCharacter.BP_FirstPersonCharacter_C|GetPlayerHUD _asbp_first_person_character)) 0.0 1 "Forward" 1.0 false)
  (Rendering|Components|TextRender|SetText (Variables|/Game/TDWidgets/UI_PlayerHUD.UI_PlayerHUD_C|GetHealthBreakText (Variables|/Game/FirstPerson/Blueprints/BP_FirstPersonCharacter.BP_FirstPersonCharacter_C|GetPlayerHUD _asbp_first_person_character)) "Prepare to battle!")
  (bind _returnvalue_2 (Utilities|Time|SetTimerbyEvent (delegate Custom|New%20Wave) (Variables|BreakVars|GetCurrentBreakLength)))
  (Variables|BreakVars|SetBreakTimer _returnvalue_2))

(event Custom|New%20Wave
  (bind _waveenemyamounts (Variables|Default|GetWaveEnemyAmounts))
  (bind _wave (Variables|Default|GetWave))
  (bind _value (Utilities|Map|Find _waveenemyamounts _wave))
  ;[1 0.3404 0.5745] Clear Break Time elements and revert User Interface by invalidating the Timer and playing the Break animation in reverse.
  (Audio|Components|Audio|FadeOut (Variables|Default|GetBreakMusic) 1.0 0.0 "Linear" :!class /Script/Engine.AudioComponent)
  (Utilities|Time|ClearandInvalidateTimerbyHandle (Variables|BreakVars|GetBreakTimer))
  (Variables|BreakVars|SetInBreak false)
  (bind _asbp_first_person_character (Utilities|Casting|CastToBP_FirstPersonCharacter (Game|GetPlayerCharacter 0)))
  (UserInterface|Animation|PlayAnimation (Variables|/Game/FirstPerson/Blueprints/BP_FirstPersonCharacter.BP_FirstPersonCharacter_C|GetPlayerHUD _asbp_first_person_character) (Variables|/Game/TDWidgets/UI_PlayerHUD.UI_PlayerHUD_C|GetBreakTimeStart (Variables|/Game/FirstPerson/Blueprints/BP_FirstPersonCharacter.BP_FirstPersonCharacter_C|GetPlayerHUD _asbp_first_person_character)) 0.0 1 "Reverse" 1.0 false)
  (Rendering|Components|TextRender|SetText (Variables|/Game/TDWidgets/UI_PlayerHUD.UI_PlayerHUD_C|GetHealthBreakText (Variables|/Game/FirstPerson/Blueprints/BP_FirstPersonCharacter.BP_FirstPersonCharacter_C|GetPlayerHUD _asbp_first_person_character)) "Gate Health")
  (Audio|PlaySoundatLocation "/Game/TDAudio/wavestarthorn.wavestarthorn" "0.000000,12800.000000,0.000000" "-90.000000,0.000000,0.000000" 1.0 1.0 0.0 "/Game/TDAudio/HornAtten.HornAtten" 0 0 0)
  (bind _returnvalue (Audio|SpawnSound2D (.OutItem (Utilities|Array|Random (Variables|Default|GetBattleMusicArray))) 0.5 1.0 0.0 0))
  (bind _output_get (Variables|Default|SetBattleMusic _returnvalue))
  (Audio|Components|Audio|FadeIn _output_get 2.0 1.0 0.0 "Linear" :!class /Script/Engine.AudioComponent)
  (bind _returnvalue_2 (Actor|GetActorOfClass "/Game/TDBlueprints/BP_ShopMenu.BP_ShopMenu_C"))
  (Actor|DestroyActor _returnvalue_2)
  ;[1 1 1] Resets variables that will determine the statistics at the end of the Wave.
  (bind _asbp_first_person_character_2 (Utilities|Casting|CastToBP_FirstPersonCharacter (Game|GetPlayerCharacter 0)))
  (Variables|Stats|SetInitialCurrency (Variables|/Game/FirstPerson/Blueprints/BP_FirstPersonCharacter.BP_FirstPersonCharacter_C|Getcurrency _asbp_first_person_character_2))
  (bind _returnvalue_3 (Actor|GetActorOfClass "/Game/TDBlueprints/BP_Gate.BP_Gate_C"))
  (Variables|Stats|SetGateHitsPrevWave (Variables|/Game/TDBlueprints/BP_Gate.BP_Gate_C|GetAmountOfGateHits _returnvalue_3))
  (Variables|Stats|SetEnemyDefeatsThisWave 0)
  ;[1 0.2517 0.4533] Calculates the Weight of the Enemy Spawn Table to be used to randomly spawn Enemies with a pre-determined set of chances.
  (for _array_element (Variables|Default|GetEnemy%20Spawn%20Table)
    (Variables|Default|SetProbabilityWeightSum (+ _array_element (Variables|Default|GetProbabilityWeightSum))))
  ;[0.2453 1 0.6703 0.38] Checks amount of Enemies that need to be removed (through either elimination or harm to the Gate) before the Wave is considered Cleared.
  (Variables|Default|SetEnemyRemovalsThisWave 0)
  (Variables|Default|SetEnemyRemovalsRequired _value)
  ;[0.2266 1 0.427 0.323] Spawns all of the enemies required to complete the Wave, with a modified For Loop creating a delay between each of the spawn nodes. This function references a weighted probability table that ensures that easier enemies (Forks) will spawn more often than other enemies.
  (Variables|Default|SetSpawnDelay (Math|Random|RandomFloatinRange 2.0 5.0))
  (Utilities|ForLoopwithDelay 1 _value (Variables|Default|GetSpawnDelay)
    (:Loop%20Body
      (CallFunction|SpawnEnemy)
      (Variables|Default|SetSpawnDelay (Math|Random|RandomFloatinRange 2.0 5.0)))))

(event Custom|EnemyDefeated
  ;[0.2442 0.6253 1 0.484] Adds to statistics upon an enemy being eliminated.
  (Math|Integer|IncrementInt (Variables|Stats|GetEnemyDefeatTotal)
    (:%20%20
      (Math|Integer|IncrementInt (Variables|Stats|GetEnemyDefeatsThisWave)
        (:%20%20
          (CallFunction|EnemyRemoved))))))

(event Custom|Wave%20Cleared
  (bind _returnvalue (Game|GetPlayerController 0))
  (Audio|Components|Audio|FadeOut (Variables|Default|GetBattleMusic) 2.0 0.0 "Linear" :!class /Script/Engine.AudioComponent)
  (bind _asbp_first_person_character (Utilities|Casting|CastToBP_FirstPersonCharacter (Game|GetPlayerCharacter 0)))
  ;[0.9289 0.6967 1 0.349] If the player has completed the final Wave, move to a different Results screen.
  (Variables|/Game/FirstPerson/Blueprints/BP_FirstPersonCharacter.BP_FirstPersonCharacter_C|SetCanPause _asbp_first_person_character false)
  (if (== (Variables|Default|GetWave) 1)
    (CallFunction|FinalResults)
    (else
      ;[0 0.8057 1 0.281] Creates Results Widget upon clearing a Wave, showing statistics such as the Cash gained and Enemies Eliminated.
      (bind _returnvalue_2 (UserInterface|CreateWidget "/Game/TDWidgets/UI_Results.UI_Results_C"))
      (UserInterface|Animation|PlayAnimation _returnvalue_2 (Variables|/Game/TDWidgets/UI_Results.UI_Results_C|GetFade _returnvalue_2) 0.0 1 "Forward" 1.0 false)
      (UserInterface|Viewport|AddtoViewport _returnvalue_2 0)
      (Input|SetInputModeUIOnly _returnvalue 0 "DoNotLock" false)
      (Variables|/Script/Engine.PlayerController|SetbShowMouseCursor _returnvalue true)
      (Input|DisableInput (Game|GetPlayerCharacter 0) _returnvalue))))

(event Custom|EnemyRemoved
  ;[0.3184 1 0.5592] Upon both elimination and attacking the Gate, we check if all the enemies in a Wave have been removed from play and will consider the Wave cleared if so.
  (bind _result (Math|Integer|IncrementInt (Variables|Default|GetEnemyRemovalsThisWave))
    (:%20%20
      (if (>= _result (Variables|Default|GetEnemyRemovalsRequired))
        (CallFunction|WaveCleared)))))

(event Custom|MakeNewWave
  (bind _wave (Variables|Default|GetWave))
  (Math|Integer|IncrementInt _wave
    (:%20%20
      (bind _asbp_first_person_character (Utilities|Casting|CastToBP_FirstPersonCharacter (Game|GetPlayerCharacter 0)))
      (Rendering|Components|TextRender|SetText (Variables|/Game/TDWidgets/UI_PlayerHUD.UI_PlayerHUD_C|GetWaveText (Variables|/Game/FirstPerson/Blueprints/BP_FirstPersonCharacter.BP_FirstPersonCharacter_C|GetPlayerHUD _asbp_first_person_character)) (Utilities|Text|ToText(String) (Utilities|String|Append "Wave " (Utilities|String|ToString(Integer) _wave))))
      (Game|SpawnActorfromClass "/Game/TDBlueprints/BP_ShopMenu.BP_ShopMenu_C" (Math|Transform|MakeTransform "1000.000000,700.000000,1000.000000" "0.000000,65.000000,0.000000" "1.000000,1.000000,1.000000") "Undefined" "MultiplyWithRoot" 0 0)
      (CallFunction|BreakTime 3e+01))))

(event Custom|FinalResults
  (bind _asbp_first_person_character (Utilities|Casting|CastToBP_FirstPersonCharacter (Game|GetPlayerCharacter 0)))
  (Input|DisableInput _asbp_first_person_character (Game|GetPlayerController 0))
  (UserInterface|Animation|PlayAnimation (Variables|/Game/FirstPerson/Blueprints/BP_FirstPersonCharacter.BP_FirstPersonCharacter_C|GetPlayerHUD _asbp_first_person_character) (Variables|/Game/TDWidgets/UI_PlayerHUD.UI_PlayerHUD_C|GetFadeIn (Variables|/Game/FirstPerson/Blueprints/BP_FirstPersonCharacter.BP_FirstPersonCharacter_C|GetPlayerHUD _asbp_first_person_character)) 0.0 1 "Reverse" 1.0 false)
  (Utilities|FlowControl|Delay 0.5)
  (Widget|RemovefromParent (Variables|/Game/FirstPerson/Blueprints/BP_FirstPersonCharacter.BP_FirstPersonCharacter_C|GetPlayerHUD _asbp_first_person_character))
  (bind _returnvalue (Sequencer|Player|CreateLevelSequencePlayer "/Game/TDSequences/FadeOut.FadeOut" (Utilities|Struct|MakeMovieSceneSequencePlaybackSettings true "(Value=0)" 2.0 0.0 false false false false false false false false)))
  (EventDispatchers|BindEventtoOnStop _returnvalue (delegate Custom|FinalResultsUI)))

(event Custom|FinalResultsUI
  (bind _returnvalue (Game|GetPlayerController 0))
  (Sequencer|Player|CreateLevelSequencePlayer "/Game/TDSequences/ResultsCameraPans.ResultsCameraPans" (Utilities|Struct|MakeMovieSceneSequencePlaybackSettings true (Utilities|Struct|MakeMovieSceneSequenceLoopCount 99999) 1.0 0.0 false false false false true false false true))
  (Utilities|Casting|CastToBP_FirstPersonCharacter (Game|GetPlayerCharacter 0))
  (bind _returnvalue_2 (UserInterface|CreateWidget "/Game/TDWidgets/UI_FinalResults.UI_FinalResults_C"))
  (UserInterface|Animation|PlayAnimation _returnvalue_2 (Variables|/Game/TDWidgets/UI_FinalResults.UI_FinalResults_C|GetFade _returnvalue_2) 0.0 1 "Forward" 1.0 false)
  (UserInterface|Viewport|AddtoViewport _returnvalue_2 0)
  (Input|SetInputModeUIOnly _returnvalue 0 "DoNotLock" false)
  (Variables|/Script/Engine.PlayerController|SetbShowMouseCursor _returnvalue true))

(event EventTick
  (params (DeltaSeconds :type Float%20%28single-precision%29))
  ;[0.7135 0.5129 0.5438 0.25] Checks if currently in a Break before proceeding with referencing
  (if (Variables|BreakVars|GetInBreak)
    ;[0.1086 0.3761 0.8281 0.224] Updates the Timer Bar in the Player's HUD based on the time remaining in the Break.
    (bind _asbp_first_person_character (Utilities|Casting|CastToBP_FirstPersonCharacter (Game|GetPlayerCharacter 0)))
    (Default|BreakTimerBar (Variables|/Game/FirstPerson/Blueprints/BP_FirstPersonCharacter.BP_FirstPersonCharacter_C|GetPlayerHUD _asbp_first_person_character) (/ (Class|KismetSystemLibrary|GetTimerElapsedTimeHandle (Variables|BreakVars|GetBreakTimer)) (Variables|BreakVars|GetCurrentBreakLength)))))

(fn ConstructionScript)

(fn SpawnEnemy
  (LocalVariables|SetRandomValue (Math|Random|RandomFloatinRange 0.0 (Variables|Default|GetProbabilityWeightSum)))
  (bind (_array_element _array_index) (Utilities|Array|ForEachLoopwithBreak (Variables|Default|GetEnemy%20Spawn%20Table) :!label _label)
    (:LoopBody
      (bind _output_get (LocalVariables|SetLocalSum (+ _array_element (LocalVariables|GetLocalSum))))
      (if (>= _output_get (LocalVariables|GetRandomValue))
        (goto _label Break)))
    (:Completed
      (Game|SpawnActorfromClass (.Value (Utilities|Map|Find (Variables|Default|GetEnemyReferences) _array_index)) (Math|Transform|MakeTransform "0.000000,12800.000000,0.000000" "0, 0, 0" "1.000000,1.000000,1.000000") "Undefined" "MultiplyWithRoot" 0 0))))