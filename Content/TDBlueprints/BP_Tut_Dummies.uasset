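; BP_Tut_Dummies is a tutorial target dummy that tips over when shot and rewards the player.
; Any hit plays a random sound, but only a BP_FirstPersonProjectile starts the Timeline that rotates the mesh down.
; When the fall finishes, it adds Currency and increments EnemiesKilled on the player character.
; The third and fourth kills update the TutorialHUD tip, pointing first to upgrades, then to the Zipline.
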(event Collision|EventHit
  (params (MyComp :type Primitive%20Component%20Object%20Reference) (Other :type Actor%20Object%20Reference) (OtherComp :type Primitive%20Component%20Object%20Reference) (bSelfMoved :type Boolean) (HitLocation :type Vector :default "0, 0, 0") (HitNormal :type Vector :default "0, 0, 0") (NormalImpulse :type Vector :default "0, 0, 0") (Hit :type Hit%20Result%20Structure%20%28by%20ref%29))
  (Audio|PlaySoundatLocation (.OutItem (Utilities|Array|Random (Variables|Default|GetHitSounds))) (Transformation|GetActorLocation) "0, 0, 0" 1.0 1.0 0.0 0 0 0 0)
  (Utilities|Casting|CastToBP_FirstPersonProjectile Other)
  (bind _dummyfall (Timeline|Timeline Play)
    (:Update
      (Transformation|SetRelativeRotation (Variables|Default|GetStaticMesh) (Math|Rotator|MakeRotator (Math|Float|Lerp 0.0 -9e+01 _dummyfall) 0.0 0.0) false false))
    (:Finished
      (bind _asbp_first_person_character (Utilities|Casting|CastToBP_FirstPersonCharacter (Game|GetPlayerCharacter 0)))
      (Variables|/Game/FirstPerson/Blueprints/BP_FirstPersonCharacter.BP_FirstPersonCharacter_C|Setcurrency _asbp_first_person_character (+ (Variables|/Game/FirstPerson/Blueprints/BP_FirstPersonCharacter.BP_FirstPersonCharacter_C|Getcurrency _asbp_first_person_character) 10))
      (bind _result (Math|Integer|IncrementInt (Variables|/Game/FirstPerson/Blueprints/BP_FirstPersonCharacter.BP_FirstPersonCharacter_C|GetEnemiesKilled _asbp_first_person_character))
        (:%20%20
          (switch int _result
            (:3
              (bind _asbp_first_person_character_2 (Utilities|Casting|CastToBP_FirstPersonCharacter (Game|GetPlayerCharacter 0)))
              (Rendering|Components|TextRender|SetText (Variables|/Game/TDWidgets/UI_TutorialHUD.UI_TutorialHUD_C|GetTipText (Variables|/Game/FirstPerson/Blueprints/BP_FirstPersonCharacter.BP_FirstPersonCharacter_C|GetTutorialHUD _asbp_first_person_character_2)) "Enemies give you Cash. To hit the fourth, purchase an Upgrade."))
            (:4
              (bind _asbp_first_person_character_3 (Utilities|Casting|CastToBP_FirstPersonCharacter (Game|GetPlayerCharacter 0)))
              (Rendering|Components|TextRender|SetText (Variables|/Game/TDWidgets/UI_TutorialHUD.UI_TutorialHUD_C|GetTipText (Variables|/Game/FirstPerson/Blueprints/BP_FirstPersonCharacter.BP_FirstPersonCharacter_C|GetTutorialHUD _asbp_first_person_character_3)) "Well done! Make your way to the Zipline and prepare for battle."))))))))

(fn ConstructionScript)