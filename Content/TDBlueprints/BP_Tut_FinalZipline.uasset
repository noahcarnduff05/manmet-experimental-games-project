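; Tutorial's final zipline, which sends the player along the line while fading out and returning to the main menu.
; The construction script places the exit by length and height and stretches a spline mesh between the endpoints.
; On entry overlap it disables move input, puts the player at the Plane and lerps the Plane to the exit by timeline.
; A FadeOut level sequence plays alongside, opening MainMenu when it stops.
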(event OnComponentBeginOverlap(EntryTrigger)
  (params (OverlappedComponent :type Primitive%20Component%20Object%20Reference) (OtherActor :type Actor%20Object%20Reference) (OtherComp :type Primitive%20Component%20Object%20Reference) (OtherBodyIndex :type Integer) (bFromSweep :type Boolean) (SweepResult :type Hit%20Result%20Structure%20%28by%20ref%29))
  (bind _plane (Variables|Default|GetPlane))
  (bind _returnvalue (Transformation|GetWorldLocation _plane))
  ;[0.6617 0.6706 1] Turn off Movement Input
  (bind _asbp_first_person_character (Utilities|Casting|CastToBP_FirstPersonCharacter OtherActor))
  (Input|SetIgnoreMoveInput (Game|GetPlayerController 0) true)
  ;[0.6617 0.6706 1] Ensure Plane is in correct position and move the Player to it.
  (Transformation|SetWorldLocation (Variables|Default|GetPlane) (Variables|Default|GetPlaneStart) false false)
  (Transformation|SetActorLocation _asbp_first_person_character (Math|Vector|MakeVector (.x _returnvalue) (.y _returnvalue) (Variables|Default|GetStartHeight)) false false)
  (bind _returnvalue_2 (Sequencer|Player|CreateLevelSequencePlayer "/Game/FadeOut.FadeOut"))
  (Sequencer|Player|Play _returnvalue_2 :!class /Script/MovieScene.MovieSceneSequencePlayer)
  (EventDispatchers|BindEventtoOnStop _returnvalue_2 (delegate Custom|Back%20to%20Menu))
  ;[0.6617 0.6706 1] Tween the Plane (and by extension Player) to the Exit Point of the zipline in 1.5 seconds.
  (bind _blend (Timeline|ZipPlaneBlend Play)
    (:Update
      (Transformation|SetWorldLocation (Variables|Default|GetPlane) (Math|Vector|Lerp(Vector) (Variables|Default|GetPlaneStart) (Variables|Default|GetPlaneExit) _blend) false false))))

(event Custom|Back%20to%20Menu
  (Game|OpenLevel(byObjectReference) "/Game/TDMaps/MainMenu.MainMenu"))

(event EventBeginPlay
  (bind _exit (Variables|Default|GetExit))
  (bind _dropoffoffset (Variables|Default|GetDropoffOffset))
  (bind _dropoffoffset_2 (Variables|Default|GetDropoffOffset))
  (bind _entry (Variables|Default|GetEntry))
  (bind _entry_2 (Variables|Default|GetEntry))
  (bind _dropoffoffset_3 (Variables|Default|GetDropoffOffset))
  (bind _exit_2 (Variables|Default|GetExit))
  (bind _returnvalue (Math|Vector|GetForwardVector _entry))
  (bind _returnvalue_2 (Transformation|GetWorldLocation _entry))
  (bind _returnvalue_3 (Transformation|GetWorldLocation _exit))
  (bind _returnvalue_4 (Math|Vector|GetForwardVector _exit))
  (bind _returnvalue_5 (Math|Vector|GetForwardVector _exit_2))
  (bind _returnvalue_6 (Transformation|GetWorldLocation _exit_2))
  (bind _returnvalue_7 (* _dropoffoffset_2 -1.0))
  (bind _returnvalue_8 (* _dropoffoffset_3 -1.0))
  (bind _returnvalue_9 (* _returnvalue_5 _returnvalue_8))
  (bind _returnvalue_10 (* _returnvalue_4 _dropoffoffset))
  (bind _returnvalue_11 (* _returnvalue _returnvalue_7))
  (bind _returnvalue_12 (+ _returnvalue_6 _returnvalue_9))
  (bind _returnvalue_13 (+ _returnvalue_3 _returnvalue_10))
  (bind _returnvalue_14 (+ _returnvalue_2 _returnvalue_11))
  ;[1 0.6363 0.6064 1 23] Initialise Dropoff Vectors for the player, based on the position of each Endpoint with an additional dropoff buffer (as to not get the player stuck in an inescapable loop.
  (Variables|Default|SetExitDropoff (Math|Vector|MakeVector (.x _returnvalue_13) (.y _returnvalue_13) (+ (Variables|Default|GetStartHeight) (Variables|Default|GetEndHeightOffset))))
  (Variables|Default|SetEntranceDropoff (Math|Vector|MakeVector (.x _returnvalue_14) (.y _returnvalue_14) (Variables|Default|GetStartHeight)))
  ;[1 0.5322 0.72] The Plane Start variable will determine where the player teleports to for the beginning of the zipline's animation with regards to how big the Dropoff Offset/Buffer is.
  (Variables|Default|SetPlaneStart (+ (Transformation|GetWorldLocation _entry_2) (* (Math|Vector|GetForwardVector _entry_2) (Variables|Default|GetDropoffOffset))))
  ;[1 0.5322 0.72] Ditto for the Plane Exit variable.
  (Variables|Default|SetPlaneExit (Math|Vector|MakeVector (.x _returnvalue_12) (.y _returnvalue_12) (.z _returnvalue_12))))

(fn ConstructionScript
  (bind _zipdistance (Variables|Default|GetZipDistance))
  (bind _entry (Variables|Default|GetEntry))
  (bind _returnvalue (Math|Vector|GetForwardVector _entry))
  (bind _returnvalue_2 (* _returnvalue _zipdistance))
  ;[1 0.5399 0.5399] Move Exit Point to the desired Zipline Length and Height.
  (Transformation|AddWorldOffset (Variables|Default|GetExit) (Math|Vector|MakeVector (.x _returnvalue_2) (.y _returnvalue_2) (Variables|Default|GetEndHeightOffset)) false false)
  ;[1 0.384 0.4238] Set Spline Positions for the actual line
  (SplineMesh|SetStartPosition (Variables|Default|GetSplineMesh) (Transformation|GetWorldLocation (Variables|Default|GetEntry)) true)
  (SplineMesh|SetEndPosition (Variables|Default|GetSplineMesh) (Transformation|GetWorldLocation (Variables|Default|GetExit)) true))