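; Second tutorial waypoint actor that introduces shooting when the player reaches it.
; A timeline moves its arrow vertically between two heights on BeginPlay.
; On player overlap it enables the character's shooting, fades in the tutorial HUD with a tip to shoot four dummies, unhides BP_Tut_Waypoint_3 and destroys itself.
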(event OnComponentBeginOverlap(Overlap)
  (params (OverlappedComponent :type Primitive%20Component%20Object%20Reference) (OtherActor :type Actor%20Object%20Reference) (OtherComp :type Primitive%20Component%20Object%20Reference) (OtherBodyIndex :type Integer) (bFromSweep :type Boolean) (SweepResult :type Hit%20Result%20Structure%20%28by%20ref%29))
  (bind _asbp_first_person_character (Utilities|Casting|CastToBP_FirstPersonCharacter OtherActor))
  (Variables|/Game/FirstPerson/Blueprints/BP_FirstPersonCharacter.BP_FirstPersonCharacter_C|SetcanShoot _asbp_first_person_character true)
  (UserInterface|Animation|PlayAnimation (Variables|/Game/FirstPerson/Blueprints/BP_FirstPersonCharacter.BP_FirstPersonCharacter_C|GetTutorialHUD _asbp_first_person_character) (Variables|/Game/TDWidgets/UI_TutorialHUD.UI_TutorialHUD_C|GetFadeIn (Variables|/Game/FirstPerson/Blueprints/BP_FirstPersonCharacter.BP_FirstPersonCharacter_C|GetTutorialHUD _asbp_first_person_character)) 0.0 1 "Forward" 1.0 false)
  (Rendering|Components|TextRender|SetText (Variables|/Game/TDWidgets/UI_TutorialHUD.UI_TutorialHUD_C|GetTipText (Variables|/Game/FirstPerson/Blueprints/BP_FirstPersonCharacter.BP_FirstPersonCharacter_C|GetTutorialHUD _asbp_first_person_character)) "Shoot with LMB or RT. Take down 4 dummies.")
  (bind _returnvalue (Actor|GetActorOfClass "/Game/TDBlueprints/BP_Tut_Waypoint_3.BP_Tut_Waypoint_3_C"))
  (Rendering|SetActorHiddenInGame _returnvalue false)
  (Actor|DestroyActor))

(event EventBeginPlay
  (bind _arrowfloat (Timeline|ArrowFloat Play)
    (:Update
      (bind _arrow (Variables|Default|GetArrow)
        (:then
          (Transformation|SetRelativeLocation _arrow (Math|Vector|MakeVector 0.0 0.0 (Math|Float|Lerp 5.5e+02 4.5e+02 _arrowfloat)) false false))
        (:else)))))

(fn ConstructionScript)

(fn NewFunction)