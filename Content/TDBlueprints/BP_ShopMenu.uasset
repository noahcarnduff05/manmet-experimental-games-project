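; BP_ShopMenu is a shop trigger that lets the player buy upgrades while within range.
; Entering its SphereColl volume sets CanBuy on the BP_FirstPersonCharacter and shows the BuyPanel prompt in that character's HUD.
; Leaving the volume clears CanBuy and collapses the panel.
; The purchase logic itself is not in this Blueprint.
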(event OnComponentBeginOverlap(SphereColl)
  (params (OverlappedComponent :type Primitive%20Component%20Object%20Reference) (OtherActor :type Actor%20Object%20Reference) (OtherComp :type Primitive%20Component%20Object%20Reference) (OtherBodyIndex :type Integer) (bFromSweep :type Boolean) (SweepResult :type Hit%20Result%20Structure%20%28by%20ref%29))
  ;[1 0.3209 0.3707] When the Player comes into range of the Menu, an interaction prompt will appear and the ability to Buy Upgrades will be enabled (and vice versa).
  (bind _asbp_first_person_character (Utilities|Casting|CastToBP_FirstPersonCharacter OtherActor))
  (Variables|/Game/FirstPerson/Blueprints/BP_FirstPersonCharacter.BP_FirstPersonCharacter_C|SetCanBuy _asbp_first_person_character true)
  (Widget|SetVisibility (Variables|/Game/TDWidgets/UI_PlayerHUD.UI_PlayerHUD_C|GetBuyPanel (Variables|/Game/FirstPerson/Blueprints/BP_FirstPersonCharacter.BP_FirstPersonCharacter_C|GetPlayerHUD _asbp_first_person_character)) "Visible"))

(event OnComponentEndOverlap(SphereColl)
  (params (OverlappedComponent :type Primitive%20Component%20Object%20Reference) (OtherActor :type Actor%20Object%20Reference) (OtherComp :type Primitive%20Component%20Object%20Reference) (OtherBodyIndex :type Integer))
  ;[1 0.3209 0.3707] When the Player comes into range of the Menu, an interaction prompt will appear and the ability to Buy Upgrades will be enabled (and vice versa).
  (bind _asbp_first_person_character (Utilities|Casting|CastToBP_FirstPersonCharacter OtherActor))
  (Variables|/Game/FirstPerson/Blueprints/BP_FirstPersonCharacter.BP_FirstPersonCharacter_C|SetCanBuy _asbp_first_person_character false)
  (Widget|SetVisibility (Variables|/Game/TDWidgets/UI_PlayerHUD.UI_PlayerHUD_C|GetBuyPanel (Variables|/Game/FirstPerson/Blueprints/BP_FirstPersonCharacter.BP_FirstPersonCharacter_C|GetPlayerHUD _asbp_first_person_character)) "Collapsed"))

(fn ConstructionScript)