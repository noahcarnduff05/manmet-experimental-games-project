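; Tower defense pizza wheel enemy that follows a random "PizzaPaths"-tagged spline and damages BP_Gate when it reaches the end.
; A timeline scaled by PathingTime drives movement and rotation along the spline, while a second, randomly paced timeline bobs the body.
; Damage plays hurt feedback and applies an overlay material at half health or below.
; Death triggers an explosion, awards player currency with a HUD animation, and delays actor destruction.
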(event Custom|Move%20Along%20Path
  (bind _spliney (Variables|Default|GetSpliney))
  (Components|Timeline|SetPlayRate (Variables|Default|GetEnemyMoving) (/ 1.0 (Variables|Default|GetPathingTime)))
  (bind _newtrack_0 (Timeline|EnemyMoving Play)
    (:Update
      (Transformation|SetActorTransform (Math|Transform|MakeTransform (Spline|GetLocationatDistanceAlongSpline _spliney (Math|Float|Lerp 0.0 (Spline|GetSplineLength _spliney) _newtrack_0) "World") (Spline|GetRotationatDistanceAlongSpline _spliney (Math|Float|Lerp 0.0 (Spline|GetSplineLength _spliney) _newtrack_0) "World") "1.000000,1.000000,1.000000")))
    (:Finished
      (Variables|Default|GetKnife
        (:then
          (bind _returnvalue (Actor|GetActorOfClass "/Game/TDBlueprints/Tutorial/BP_Gate.BP_Gate_C"))
          (Default|HurtGate _returnvalue (Variables|Default|GetGateDamage) (Variables|Default|GetEnemyName))
          (Actor|DestroyActor))
        (:else)))))

(event EventBeginPlay
  (Variables|Default|SetMaxHealth (Variables|Default|GetHealth))
  (bind _outactors (Actor|GetAllActorswithTag "PizzaPaths"))
  (Variables|Default|SetSpliney (Actor|GetComponentbyClass (.OutItem (Utilities|Array|Random _outactors)) "/Script/Engine.SplineComponent"))
  (CallFunction|MoveAlongPath)
  (bind _output_get (Variables|Default|SetBounceSpeed (Math|Random|RandomFloatinRange 0.9 1.2)))
  (Components|Timeline|SetPlayRate (Variables|Default|GetTimeline) _output_get)
  (bind _bounce (Timeline|Timeline Play)
    (:Update
      (Transformation|SetRelativeLocation (Variables|Default|GetBodyBox) (Math|Vector|MakeVector 0.0 0.0 (.z (Math|Vector|Lerp(Vector) "0.000000,0.000000,160.000000" "0.000000,0.000000,200.000000" _bounce))) false false))))

(event Game|Damage|EventAnyDamage
  (params (Damage :type Float%20%28single-precision%29) (DamageType :type Damage%20Type%20Object%20Reference) (InstigatedBy :type Controller%20Object%20Reference) (DamageCauser :type Actor%20Object%20Reference))
  (bind _knife (Variables|Default|GetKnife))
  (bind _output_get (Variables|Default|SetHealth (- (Variables|Default|GetHealth) Damage)))
  (if (<= _output_get 0.0)
    (Audio|Components|Audio|Stop (Variables|Default|GetTimeline))
    (Effects|SpawnEmitteratLocation "/Game/StarterContent/Particles/P_Explosion.P_Explosion" (Transformation|GetWorldLocation (Variables|Default|GetHeadBox)))
    (Audio|PlaySoundatLocation "/Game/TDAudio/enemykill.enemykill" (Transformation|GetWorldLocation (Variables|Default|GetKnife)) "0, 0, 0" 1.0 1.0 0.0 "/Game/TDAudio/EnemyHitAtten.EnemyHitAtten" 0 0 0)
    (bind _asbp_first_person_character (Utilities|Casting|CastToBP_FirstPersonCharacter (Game|GetPlayerCharacter 0)))
    (Variables|/Game/FirstPerson/Blueprints/BP_FirstPersonCharacter.BP_FirstPersonCharacter_C|Setcurrency _asbp_first_person_character (+ (Variables|/Game/FirstPerson/Blueprints/BP_FirstPersonCharacter.BP_FirstPersonCharacter_C|Getcurrency _asbp_first_person_character) 5))
    (UserInterface|Animation|PlayAnimation (Variables|/Game/FirstPerson/Blueprints/BP_FirstPersonCharacter.BP_FirstPersonCharacter_C|GetPlayerHUD _asbp_first_person_character) (Variables|/Game/TDWidgets/UI_PlayerHUD.UI_PlayerHUD_C|GetMoneyGet (Variables|/Game/FirstPerson/Blueprints/BP_FirstPersonCharacter.BP_FirstPersonCharacter_C|GetPlayerHUD _asbp_first_person_character)) 0.0 1 "Forward" 1.0 false)
    (Components|DestroyComponent (Variables|Default|GetBodyBox))
    (Utilities|FlowControl|Delay 3.0)
    (Actor|DestroyActor)
    (else
      (Audio|PlaySoundatLocation "/Game/TDAudio/enemyhurt.enemyhurt" (Transformation|GetWorldLocation (Variables|Default|GetKnife)) "0, 0, 0" 1.0 1.0 0.0 "/Game/TDAudio/EnemyHitAtten.EnemyHitAtten" 0 0 0)
      ;[1 0 0.1986 0.391] If the enemy is equal to or under half of its maximum health, an Overlay Material is applied. This can let the player strategise and prioritise different enemies in high-density waves.
      (if (<= _output_get (/ (Variables|Default|GetMaxHealth) 2.0))
        (Variables|/Script/Engine.MeshComponent|GetOverlayMaterial _knife
          (:then)
          (:else
            (Rendering|Material|SetOverlayMaterial _knife "/Game/TDMaterials/OM_HalfHealth.OM_HalfHealth" :!class /Script/Engine.MeshComponent)))))))

(fn ConstructionScript)